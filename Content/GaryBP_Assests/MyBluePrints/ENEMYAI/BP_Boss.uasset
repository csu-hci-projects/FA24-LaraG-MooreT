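; Boss enemy that fires projectiles and loses health when hit by first-person projectiles.
; BeginPlay attaches its gun to the mesh's grip socket and flags the skeleton AnimBlueprint as rifle-armed.
; StartShoot re-triggers itself by timer, spawning a projectile with sound and montage.
; At zero health it increments the player's TargetsHit, plays a death montage, destroys itself and shows the end screen with music on GMap2.
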(event Custom|Start%20Shoot
  (bind _body (Variables|Components|GetBody))
  (bind _projectileoffset (Variables|Default|GetProjectileOffset))
  (bind _returnvalue (Components|GetOwner _body))
  (bind _returnvalue_2 (Transformation|GetActorLocation _returnvalue))
  (bind _returnvalue_3 (Transformation|GetActorRotation _returnvalue))
  (bind _returnvalue_4 (Math|Vector|RotateVector _projectileoffset _returnvalue_3))
  (bind _returnvalue_5 (+ _returnvalue_2 _returnvalue_4))
  ;[1 1 1] Boss SHooting
  (Utilities|FlowControl|Delay 0.2)
  (Utilities|Time|SetTimerbyEvent (delegate Custom|Start%20Shoot) 1.0 true false 1.0)
  (Game|SpawnActorfromClass "/Game/FirstPerson/Blueprints/BP_FirstPersonProjectile.BP_FirstPersonProjectile_C" (Math|Transform|MakeTransform _returnvalue_5 _returnvalue_3) "Undefined" "OverrideRootScale" 0 0)
  (Audio|PlaySoundatLocation "/Game/FPWeapon/Audio/FirstPersonTemplateWeaponFire02.FirstPersonTemplateWeaponFire02" _returnvalue_5 "0, 0, 0" 1.0 1.0 0.0 0 0 0 0) ; Play firing sound
  (Animation|Montage|MontagePlay (Variables|Default|GetAs%20Minionby%20Garyskel%20Skeleton%20Anim%20Blueprint) "/Game/GaryBP_Assests/MyBluePrints/Mesh/Minion_anim/minionbyGaryskel_Skeleton_Montage.minionbyGaryskel_Skeleton_Montage" 1.0 "MontageLength" 0.0 true))

(event EventBeginPlay
  ;[1 1 1] Attach gun to boss hands
  (Transformation|AttachComponentToComponent (Variables|Actor|GetGun) (Variables|Character|GetMesh) "GripPoint" "SnapToTarget" "SnapToTarget" "SnapToTarget" true)
  (bind _asminionby_garyskel_skeleton_anim_blueprint (Utilities|Casting|CastTominionbyGaryskel_Skeleton_AnimBlueprint (Components|SkeletalMesh|GetAnimInstance (Variables|Character|GetMesh))))
  (bind _output_get (Variables|Default|SetAs%20Minionby%20Garyskel%20Skeleton%20Anim%20Blueprint _asminionby_garyskel_skeleton_anim_blueprint))
  (Variables|/Game/GaryBP_Assests/MyBluePrints/Mesh/Minion_anim/minionbyGaryskel_Skeleton_AnimBlueprint.minionbyGaryskel_Skeleton_AnimBlueprint_C|SetHasRifle _output_get true))

(event Collision|EventHit
  (params (MyComp :type Primitive%20Component%20Object%20Reference) (Other :type Actor%20Object%20Reference) (OtherComp :type Primitive%20Component%20Object%20Reference) (bSelfMoved :type Boolean) (HitLocation :type Vector :default "0, 0, 0") (HitNormal :type Vector :default "0, 0, 0") (NormalImpulse :type Vector :default "0, 0, 0") (Hit :type Hit%20Result%20Structure%20%28by%20ref%29))
  ;[1 1 1] Lower Boss health when shot
  (Utilities|Casting|CastToBP_FirstPersonProjectile Other)
  (Variables|Default|SetBoss%20Health (- (Variables|Default|GetBoss%20Health) 1))
  (if (<= (Variables|Default|GetBoss%20Health) 0)
    (bind _asbp_first_person_character (Utilities|Casting|CastToBP_FirstPersonCharacter (Game|GetPlayerCharacter 0)))
    (Variables|/Game/FirstPerson/Blueprints/BP_FirstPersonCharacter.BP_FirstPersonCharacter_C|SetTargets%20Hit _asbp_first_person_character (+ (Variables|/Game/FirstPerson/Blueprints/BP_FirstPersonCharacter.BP_FirstPersonCharacter_C|GetTargets%20Hit _asbp_first_person_character) 1))
    (Animation|Montage|MontagePlay (Variables|Default|GetAs%20Minionby%20Garyskel%20Skeleton%20Anim%20Blueprint) "/Game/GaryBP_Assests/MyBluePrints/Mesh/Minion_anim/miniondeath.miniondeath" 1.0 "MontageLength" 0.0 true)
    (Utilities|FlowControl|Delay 1.2)
    (Actor|DestroyActor)
    (|SetEndScreen)))

(fn ConstructionScript)